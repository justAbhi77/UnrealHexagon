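; BP_PlayerActions handles tile hover highlighting on a placement grid for the local player, enabling input from player controller 0 at startup.
; Every tick it asks the referenced grid for the tile index under the cursor.
; When that index changes, it looks up the old and new tiles in the grid's Tiles map, unhighlights the old, highlights the new, then caches the new index.
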(event EventBeginPlay
  (Input|EnableInput (Game|GetPlayerController 0)))

(event EventTick
  (params (DeltaSeconds :type Float%20%28single-precision%29))
  (CallFunction|FUpdateTile))

(fn ConstructionScript)

(fn FUpdateTile
  (Utilities|FlowControl|Sequence
    (:then_0
      (bind _gridplacementref (Variables|Default|GetGridPlacementRef)
        (:then
          (bind _index (Default|FGetTileIndexUnderCursor _gridplacementref))
          (LocalVariables|SetNewIndex _index))
        (:else)))
    (:then_1
      (if (!= (LocalVariables|GetNewIndex) (Variables|Default|GetIndex))
        (Utilities|FlowControl|Sequence
          (:then_0
            (bind _gridplacementref_2 (Variables|Default|GetGridPlacementRef)
              (:then
                (if (.ReturnValue (Utilities|Map|Find (Variables|/Game/Blueprints/BP_GridPlacement.BP_GridPlacement_C|GetTiles _gridplacementref_2) (Variables|Default|GetIndex)))
                  (Default|FUnHighlightTile (.Value (Utilities|Map|Find (Variables|/Game/Blueprints/BP_GridPlacement.BP_GridPlacement_C|GetTiles _gridplacementref_2) (Variables|Default|GetIndex))))))
              (:else)))
          (:then_1
            (bind _gridplacementref_3 (Variables|Default|GetGridPlacementRef)
              (:then
                (if (.ReturnValue (Utilities|Map|Find (Variables|/Game/Blueprints/BP_GridPlacement.BP_GridPlacement_C|GetTiles _gridplacementref_3) (LocalVariables|GetNewIndex)))
                  (Default|FHighlightTile (.Value (Utilities|Map|Find (Variables|/Game/Blueprints/BP_GridPlacement.BP_GridPlacement_C|GetTiles _gridplacementref_3) (LocalVariables|GetNewIndex))))))
              (:else)))
          (:then_2
            (Variables|Default|SetIndex (LocalVariables|GetNewIndex))))))))