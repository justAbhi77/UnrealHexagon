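; BFL_Utilities is a Blueprint function library of small, independent helpers for math and runtime checks.
; It snaps one vector to per-axis grid sizes from another and tests floats or integers for evenness.
; It also rolls a random integer between a paired min and max in either order.
; The in-game check passes when either player controller 0 or the game mode is valid.
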(fn FSnapVectortoVector
  (params (V1 :type Vector) (V2 :type Vector))
  (return (Math|Vector|MakeVector (Math|Float|SnapToGrid(Float) (.x V1) (.x V2)) (Math|Float|SnapToGrid(Float) (.y V1) (.y V2)) (Math|Float|SnapToGrid(Float) (.z V1) (.z V2)))))

(fn FIsFloatEven
  (params (Float :type Float%20%28double-precision%29))
  (return (== (Math|Float|%(Float) Float 2.0) 0.0)))

(fn FIsIntEven
  (params (Int :type Integer))
  (return (== (Math|Integer|%(Integer) Int 2) 0)))

(fn FMinMaxRandom
  (params (MInMax :type Int%20Point%20Structure))
  (if (<= (.x MInMax) (.y MInMax))
    (return (Math|Random|RandomIntegerinRange (.x MInMax) (.y MInMax)))
    (else
      (return (Math|Random|RandomIntegerinRange (.y MInMax) (.x MInMax))))))

(fn FIsinGame
  (return (or (Utilities|IsValid (Game|GetPlayerController 0)) (Utilities|IsValid (Game|GetGameMode)))))