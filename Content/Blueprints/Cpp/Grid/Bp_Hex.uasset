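; Bp_Hex is a hex grid tile that displays its coordinates and changes color when highlighted.
; On BeginPlay it creates a dynamic material instance from MHexBase on the tile mesh, tints it with TileColor and writes TileCoordinates to a debug text component.
; Highlight and unhighlight events switch that material's Color parameter between a fixed red-pink and TileColor.
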(event EventOnTileHighlighted
  (bind _basemat (Variables|Default|GetBaseMat)
    (:then
      (Rendering|Material|SetVectorParameterValue _basemat "Color" "(R=1.000000,G=0.000000,B=0.168269,A=1.000000)" :!class /Script/Engine.MaterialInstanceDynamic))
    (:else)))

(event EventOnTileUnHighlighted
  (bind _basemat (Variables|Default|GetBaseMat)
    (:then
      (Rendering|Material|SetVectorParameterValue _basemat "Color" (Variables|Default|GetTileColor) :!class /Script/Engine.MaterialInstanceDynamic))
    (:else)))

(event EventBeginPlay
  (|CallParentFunction)
  (bind _returnvalue (Rendering|Material|CreateDynamicMaterialInstance (Variables|Default|GetSmTile) 0 "/Game/Assets/Materials/MHexBase.MHexBase" "None" :!class /Script/Engine.PrimitiveComponent))
  (bind _output_get (Variables|Default|SetBaseMat _returnvalue))
  (Rendering|Material|SetVectorParameterValue _output_get "Color" (Variables|Default|GetTileColor) :!class /Script/Engine.MaterialInstanceDynamic)
  (Rendering|Components|TextRender|SetText (Variables|Default|GetTr_Debug) (Utilities|Text|ToText(String) (Utilities|String|ToString(Integer) (Variables|Default|GetTileCoordinates)))))

(fn ConstructionScript)