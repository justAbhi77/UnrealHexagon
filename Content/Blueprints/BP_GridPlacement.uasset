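; Grid actor that builds a hexagon-shaped board of resource tiles with settlement and road spots, in the style of Catan.
; BeginPlay shuffles a tile-type pool from TileMapCount, then spawns BP_Tile actors on doubled-row indices, with water around the rim.
; Each hex spawns corner BP_Settlements and edge BP_Roads, deduplicated by scaled vertex key and edge midpoint, under organizing parent actors.
; Helpers convert mouse ray-plane hits to tile indices.
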(event EventBeginPlay
  (bind _hexagonsize (Variables|Default|GetHexagonSize))
  (bind _returnvalue (* _hexagonsize 2))
  (bind _returnvalue_2 (- _returnvalue 1))
  (Utilities|FlowControl|Sequence
    (:then_0
      (bind _keys (Utilities|Map|Keys (Variables|Default|GetTileMapCount)))
      (for _array_element _keys
        (for _index (range 1 (.Value (Utilities|Map|Find (Variables|Default|GetTileMapCount) _array_element)))
          (Utilities|Array|Add (Variables|Default|GetBoardTilesCount) _array_element)))
      (Utilities|Array|Shuffle (Variables|Default|GetBoardTilesCount)))
    (:then_1
      (CallFunction|FGenerateGrid (Transformation|GetActorLocation) (Variables|Default|GetGrid%20Tile%20Size) (Utilities|Struct|MakeIntPoint _returnvalue_2 _returnvalue_2)))))

(fn ConstructionScript
  (bind _hexagonsize (Variables|Default|GetHexagonSize))
  (bind _returnvalue (* _hexagonsize 2))
  (bind _returnvalue_2 (- _returnvalue 1))
  (Variables|Default|ForDevEyesOnly|SetGrid%20Tile%20Count (Utilities|Struct|MakeIntPoint _returnvalue_2 _returnvalue_2)))

(fn FGenerateGrid
  (params (CenterLocation :type Vector) (TileSize :type Vector) (Grid%20Tile%20Count :type Int%20Point%20Structure))
  (bind _ybounds (LocalVariables|GetYBounds))
  (bind _ybounds_2 (LocalVariables|GetYBounds))
  (bind (_x _y) (Utilities|Struct|BreakIntPoint _ybounds))
  (Variables|Default|SetGrid%20Center%20Location CenterLocation)
  (Variables|Default|SetGrid%20Tile%20Size TileSize)
  (Variables|Default|ForDevEyesOnly|SetGrid%20Tile%20Count Grid%20Tile%20Count)
  (Utilities|FlowControl|Sequence
    (:then_0
      (Utilities|FlowControl|Sequence
        (:then_0
          (bind _returnvalue (CallFunction|FSpawnCleanHierarchicalActors))
          (Variables|Default|SetCleanHierarchyWorldTiles _returnvalue))
        (:then_1
          (bind _returnvalue_2 (CallFunction|FSpawnCleanHierarchicalActors))
          (Variables|Default|SetCleanHierarchyWorldSettlements _returnvalue_2))
        (:then_2
          (bind _returnvalue_3 (CallFunction|FSpawnCleanHierarchicalActors))
          (Variables|Default|SetCleanHierarchyWorldRoads _returnvalue_3))))
    (:then_1
      (CallFunction|FDestroyGrid)
      (bind (_center _bottomleft) (CallFunction|FCalculateCenterandBottomLeft))
      (Variables|Default|SetGrid%20Center%20Location _center)
      (Variables|Default|SetGrid%20Bottom%20Left%20Corner%20Location _bottomleft)
      (for _index (range 0 (- (.x (Variables|Default|ForDevEyesOnly|GetGrid%20Tile%20Count)) 1))
        (bind _output_get (LocalVariables|SetX _index))
        (|SetBy-RefVar _x (.FirstIndex (CallFunction|FGetWorldTileYIndex _output_get)))
        (|SetBy-RefVar _y (.LastIndex (CallFunction|FGetWorldTileYIndex _output_get)))
        (for _index_2 (range (.x _ybounds_2) (.y _ybounds_2))
          (LocalVariables|SetY _index_2)
          (Utilities|FlowControl|Sequence
            (:then_0
              (LocalVariables|SetIndex (Utilities|Struct|MakeIntPoint (LocalVariables|GetX) (LocalVariables|GetY)))
              (LocalVariables|SetTileTransform (Math|Transform|MakeTransform (CallFunction|FGetTileLocationfromGridIndex (LocalVariables|GetIndex)) (CallFunction|FGetTileRotationfromGridIndex (LocalVariables|GetIndex)) (CallFunction|FGetTileScale)))
              (CallFunction|FAddGridTile (LocalVariables|GetIndex) (LocalVariables|GetTileTransform) (LocalVariables|GetYBounds))
              (CallFunction|FGenerateVerticesandEdgesforHexagon (LocalVariables|GetIndex)))
            (:then_1
              (Math|Integer|IncrementInt _index_2))))))))

(fn FDestroyGrid
  (Utilities|FlowControl|Sequence
    (:then_0
      (bind _values (Utilities|Map|Values (Variables|Default|GetTiles)))
      (for _array_element _values
        (Utilities|IsValid _array_element
          (:Is%20Valid
            (Actor|DestroyActor _array_element))))
      (Utilities|Map|Clear (Variables|Default|GetTiles)))
    (:then_2
      (Utilities|Map|Clear (Variables|Default|GetSettlement_ChildActor)))
    (:then_3
      (Utilities|Map|Clear (Variables|Default|GetRoads_ChildActor))
      (Utilities|Array|Clear (Variables|Default|GetRoads)))))

(fn FCalculateCenterandBottomLeft
  (Utilities|FlowControl|Sequence
    (:then_0
      (LocalVariables|SetC (CallFunction|FSnapVectortoVector (Variables|Default|GetGrid%20Center%20Location) (Variables|Default|GetGrid%20Tile%20Size)))
      (LocalVariables|SetBL (- (LocalVariables|GetC) (CallFunction|FSnapVectortoVector (* (Variables|Default|GetGrid%20Tile%20Size) (Math|Conversions|ToVector(Vector2D) (/ (Variables|Default|ForDevEyesOnly|GetGrid%20Tile%20Count) "(X=3.000000,Y=3.000000)"))) (Variables|Default|GetGrid%20Tile%20Size)))))
    (:then_1
      (return (LocalVariables|GetC) (LocalVariables|GetBL)))))

(fn FGetWorldTileYIndex
  (params (X :type Integer))
  (bind _grid_tile_count (Variables|Default|ForDevEyesOnly|GetGrid%20Tile%20Count))
  (bind _grid_tile_count_2 (Variables|Default|ForDevEyesOnly|GetGrid%20Tile%20Count))
  (bind _grid_tile_count_3 (Variables|Default|ForDevEyesOnly|GetGrid%20Tile%20Count))
  (bind _returnvalue (* (.y _grid_tile_count_2) 2))
  (bind _returnvalue_2 (* X 2))
  (bind _returnvalue_3 (+ (.x _grid_tile_count) 1))
  (bind _returnvalue_4 (+ _returnvalue_2 1))
  (bind _returnvalue_5 (/ _returnvalue_3 2))
  (bind _returnvalue_6 (- _returnvalue 1))
  (bind _biseven (CallFunction|FIsIntEven _returnvalue_5))
  (bind _returnvalue_7 (- (.x _grid_tile_count_3) _returnvalue_4))
  (bind _returnvalue_8 (/ _returnvalue_7 2))
  (bind _returnvalue_9 (Math|Integer|Absolute(Integer) _returnvalue_8))
  (bind _biseven_2 (CallFunction|FIsIntEven _returnvalue_9))
  (bind _returnvalue_10 (+ _returnvalue_9 1))
  (bind _returnvalue_11 (- _returnvalue_9 1))
  (bind _returnvalue_12 (Math|Integer|SelectInt _returnvalue_9 _returnvalue_11 _biseven_2))
  (bind _returnvalue_13 (- _returnvalue_6 _returnvalue_12))
  (return (Math|Integer|SelectInt _returnvalue_10 (- _returnvalue_10 1) _biseven) (Math|Integer|SelectInt _returnvalue_13 (- _returnvalue_13 1) _biseven)))

(fn FGetTileLocationfromGridIndex
  (params (GridIndex :type Int%20Point%20Structure))
  (return (+ (Variables|Default|GetGrid%20Bottom%20Left%20Corner%20Location) (* (Math|Conversions|ToVector(Vector2D) (* GridIndex "(X=0.750000,Y=0.500000)")) (Variables|Default|GetGrid%20Tile%20Size)))))

(fn FGetTileRotationfromGridIndex
  (params (GridIndex :type Int%20Point%20Structure))
  (return (LocalVariables|GetReturnRotation)))

(fn FGetTileScale
  (return (/ (Variables|Default|GetGrid%20Tile%20Size) (Variables|Default|GetMeshSize))))

(fn FAddGridTile
  (params (Index :type Int%20Point%20Structure) (Transform :type Transform) (YBounds :type Int%20Point%20Structure))
  (bind _tiles (Variables|Default|GetTiles))
  (bind (_value _returnvalue) (Utilities|Map|Find _tiles Index))
  (Utilities|FlowControl|Sequence
    (:then_0
      (LocalVariables|SetbIsWaterTile (Math|Boolean|ORBoolean (== (.x Index) 0) (== (.x Index) (- (.x (Variables|Default|ForDevEyesOnly|GetGrid%20Tile%20Count)) 1)) (== (.y Index) (.x YBounds)) (== (.y YBounds) (.y Index)) (== (.y Index) (- (.y YBounds) 1)))))
    (:then_1
      (if _returnvalue
        (Transformation|SetWorldTransform (Variables|/Game/Blueprints/BP_Tile.BP_Tile_C|GetDefaultSceneRoot _value) Transform false false)
        (LocalVariables|SetCurrentTile _value)
        (else
          (bind _returnvalue_2 (Game|SpawnActorfromClass "/Game/Blueprints/BP_Tile.BP_Tile_C" Transform "AlwaysSpawn" "MultiplyWithRoot" self (Math|Conversions|ToVector2D(IntPoint) Index) 0))
          (bind _output_get (LocalVariables|SetCurrentTile _returnvalue_2))
          (Utilities|Map|Add (Variables|Default|GetTiles) Index _output_get)
          (Transformation|AttachActorToActor (LocalVariables|GetCurrentTile) (Variables|Default|GetCleanHierarchyWorldTiles) "None" "KeepRelative" "KeepRelative" "KeepRelative" true))))
    (:then_2
      (Default|FSetupTileProperties (LocalVariables|GetCurrentTile) (LocalVariables|GetbIsWaterTile) (select (LocalVariables|GetbIsWaterTile) "NewEnumerator6" (Utilities|Array|Get(acopy) (Variables|Default|GetBoardTilesCount) (Math|Integer|%(Integer) (Variables|Default|GetArrayIndex) (Utilities|Array|Length (Variables|Default|GetBoardTilesCount))))) (.Value (Utilities|Map|Find (Variables|Default|GetTileMap) (select (LocalVariables|GetbIsWaterTile) "NewEnumerator6" (Utilities|Array|Get(acopy) (Variables|Default|GetBoardTilesCount) (Math|Integer|%(Integer) (Variables|Default|GetArrayIndex) (Utilities|Array|Length (Variables|Default|GetBoardTilesCount))))))) (Utilities|Select :Index (select (LocalVariables|GetbIsWaterTile) "NewEnumerator6" (Utilities|Array|Get(acopy) (Variables|Default|GetBoardTilesCount) (Math|Integer|%(Integer) (Variables|Default|GetArrayIndex) (Utilities|Array|Length (Variables|Default|GetBoardTilesCount))))) :NewEnumerator0 "/Game/Assets/Models/sand-desert_sand_desert.sand-desert_sand_desert" :NewEnumerator1 "/Game/Assets/Models/stone-rocks_stone_rocks.stone-rocks_stone_rocks" :NewEnumerator2 "/Game/Assets/Models/grass-forest_grass_forest.grass-forest_grass_forest" :NewEnumerator3 "/Game/Assets/Models/stone-mountain_stone_mountain.stone-mountain_stone_mountain" :NewEnumerator4 "/Game/Assets/Models/building-smelter_building_smelter.building-smelter_building_smelter" :NewEnumerator5 "/Game/Assets/Models/building-sheep_building_sheep.building-sheep_building_sheep" :NewEnumerator6 "/Game/Assets/Models/water_water.water_water") (select (LocalVariables|GetbIsWaterTile) "/Game/Assets/Materials/MM_Base.MM_Base" "/Game/Assets/Materials/MM_Base.MM_Base"))
      (if (not (LocalVariables|GetbIsWaterTile))
        (Math|Integer|IncrementInt (Variables|Default|GetArrayIndex))))))

(fn FGetHexagonVertexIndicesfromGridIndex
  (params (GridIndex :type Int%20Point%20Structure))
  (bind _returnvalue (* GridIndex "(X=0.750000,Y=0.500000)"))
  (return (Utilities|Array|MakeArray (+ _returnvalue "(X=0.500000,Y=0.000000)") (+ _returnvalue "(X=0.250000,Y=0.500000)") (+ _returnvalue "(X=-0.250000,Y=0.500000)") (+ _returnvalue "(X=-0.500000,Y=0.000000)") (+ _returnvalue "(X=-0.250000,Y=-0.500000)") (+ _returnvalue "(X=0.250000,Y=-0.500000)"))))

(fn FGetVertexLocationfromVertexIndex
  (params (VertexIndex :type Vector%202D%20Structure) (Z :type Float%20%28single-precision%29))
  (return (+ (Variables|Default|GetGrid%20Bottom%20Left%20Corner%20Location) (* (Math|Conversions|ToVector(Vector2D) VertexIndex Z) (Variables|Default|GetGrid%20Tile%20Size)))))

(fn FGetHexagonVertexIndicesfromGridIndexNew
  (params (CellCenter :type Vector) (CellRadius :type Float%20%28double-precision%29))
  (for _index (range 0 5)
    (Utilities|Array|Add (LocalVariables|GetArray) (Math|Vector2D|MakeVector2D (+ (.x CellCenter) (* (Math|Trig|Cos(Degrees) (* _index 6e+01)) CellRadius)) (+ (.y CellCenter) (* (Math|Trig|Sin(Degrees) (* _index 6e+01)) CellRadius)))))
  (return (LocalVariables|GetArray)))

(fn FGenerateVerticesandEdgesforHexagon
  (params (Index :type Int%20Point%20Structure))
  (bind _output_get (LocalVariables|SetVertices (CallFunction|FGetHexagonVertexIndicesfromGridIndex Index)))
  (LocalVariables|SetArrayLength (Utilities|Array|Length _output_get))
  (for _index (range 0 (- (Utilities|Array|Length _output_get) 1))
    (LocalVariables|SetCurrentVertexIndex _index)
    (LocalVariables|SetCurrentVertex (Utilities|Array|Get(acopy) (LocalVariables|GetVertices) (LocalVariables|GetCurrentVertexIndex)))
    (Utilities|FlowControl|Sequence
      (:then_0
        (Utilities|FlowControl|Sequence
          (:then_0
            (LocalVariables|SetCurrentVertexLocation (CallFunction|FGetVertexLocationfromVertexIndex (LocalVariables|GetCurrentVertex) 1.1)))
          (:then_1
            (if (not (.ReturnValue (Utilities|Map|Find (Variables|Default|GetSettlement_ChildActor) (* (LocalVariables|GetCurrentVertex) "(X=8.000000,Y=4.000000)"))))
              (bind _returnvalue (Game|SpawnActorfromClass "/Game/Blueprints/BP_Settlement.BP_Settlement_C" (Math|Transform|MakeTransform (LocalVariables|GetCurrentVertexLocation) "0, 0, 0" "0.200000,0.200000,0.200000") "AlwaysSpawn" "MultiplyWithRoot" self (* (LocalVariables|GetCurrentVertex) "(X=8.000000,Y=4.000000)") 0))
              (Utilities|Map|Add (Variables|Default|GetSettlement_ChildActor) (* (LocalVariables|GetCurrentVertex) "(X=8.000000,Y=4.000000)") _returnvalue)
              (Transformation|AttachActorToActor _returnvalue (Variables|Default|GetCleanHierarchyWorldSettlements) "None" "KeepRelative" "KeepRelative" "KeepRelative" true)))
          (:then_2
            (if (Utilities|Array|IsValidIndex (LocalVariables|GetVertices) (Math|Integer|%(Integer) (+ (LocalVariables|GetCurrentVertexIndex) 1) (LocalVariables|GetArrayLength)))
              (if (not (Utilities|Array|ContainsItem (Variables|Default|GetRoads) (Math|Vector|Lerp(Vector) (LocalVariables|GetCurrentVertexLocation) (CallFunction|FGetVertexLocationfromVertexIndex (Utilities|Array|Get(acopy) (LocalVariables|GetVertices) (Math|Integer|%(Integer) (+ (LocalVariables|GetCurrentVertexIndex) 1) (LocalVariables|GetArrayLength))) 1.1) 0.5)))
                (Utilities|Array|Add (Variables|Default|GetRoads) (Math|Vector|Lerp(Vector) (LocalVariables|GetCurrentVertexLocation) (CallFunction|FGetVertexLocationfromVertexIndex (Utilities|Array|Get(acopy) (LocalVariables|GetVertices) (Math|Integer|%(Integer) (+ (LocalVariables|GetCurrentVertexIndex) 1) (LocalVariables|GetArrayLength))) 1.1) 0.5))
                (bind _returnvalue_2 (Game|SpawnActorfromClass "/Game/Blueprints/BP_Road.BP_Road_C" (Math|Transform|MakeTransform (Math|Vector|Lerp(Vector) (LocalVariables|GetCurrentVertexLocation) (CallFunction|FGetVertexLocationfromVertexIndex (Utilities|Array|Get(acopy) (LocalVariables|GetVertices) (Math|Integer|%(Integer) (+ (LocalVariables|GetCurrentVertexIndex) 1) (LocalVariables|GetArrayLength))) 1.1) 0.5) (Math|Rotator|FindLookatRotation (LocalVariables|GetCurrentVertexLocation) (CallFunction|FGetVertexLocationfromVertexIndex (Utilities|Array|Get(acopy) (LocalVariables|GetVertices) (Math|Integer|%(Integer) (+ (LocalVariables|GetCurrentVertexIndex) 1) (LocalVariables|GetArrayLength))) 1.1)) (Math|Vector|MakeVector (Math|Vector|Distance(Vector) (LocalVariables|GetCurrentVertexLocation) (CallFunction|FGetVertexLocationfromVertexIndex (Utilities|Array|Get(acopy) (LocalVariables|GetVertices) (Math|Integer|%(Integer) (+ (LocalVariables|GetCurrentVertexIndex) 1) (LocalVariables|GetArrayLength))) 1.1)) 5.0 1.0)) "AlwaysSpawn" "MultiplyWithRoot" self (* (+ (LocalVariables|GetCurrentVertex) (Utilities|Array|Get(acopy) (LocalVariables|GetVertices) (Math|Integer|%(Integer) (+ (LocalVariables|GetCurrentVertexIndex) 1) (LocalVariables|GetArrayLength)))) "(X=4.000000,Y=2.000000)") 0))
                (Utilities|Map|Add (Variables|Default|GetRoads_ChildActor) (* (+ (LocalVariables|GetCurrentVertex) (Utilities|Array|Get(acopy) (LocalVariables|GetVertices) (Math|Integer|%(Integer) (+ (LocalVariables|GetCurrentVertexIndex) 1) (LocalVariables|GetArrayLength)))) "(X=4.000000,Y=2.000000)") _returnvalue_2)
                (Transformation|AttachActorToActor _returnvalue_2 (Variables|Default|GetCleanHierarchyWorldRoads) "None" "KeepRelative" "KeepRelative" "KeepRelative" true)))))))))

(fn FSpawnCleanHierarchicalActors
  (bind _returnvalue (Game|SpawnActorfromClass "/Script/Engine.Actor" (Transformation|GetActorTransform) "AlwaysSpawn" "MultiplyWithRoot" self 0))
  (bind _output_get (LocalVariables|SetSpawnedActor _returnvalue))
  (AddComponent|AddSceneComponent _output_get false)
  (Transformation|AttachActorToActor (LocalVariables|GetSpawnedActor) self "None" "SnapToTarget" "SnapToTarget" "SnapToTarget" true)
  (return (LocalVariables|GetSpawnedActor)))

(fn FGetTileIndexUnderCursor
  (params (PlayerIndex :type Integer))
  (bind _location (CallFunction|FGetCursorLocationonGrid PlayerIndex))
  (bind _index (CallFunction|FGetTileIndexfromWorldLocation _location))
  (return _index))

(fn FGetCursorLocationonGrid
  (params (PlayerIndex :type Integer))
  (bind _grid_center_location (Variables|Default|GetGrid%20Center%20Location))
  (bind _returnvalue (Game|GetPlayerController PlayerIndex))
  (bind _returnvalue_2 (Class|KismetMathLibrary|MakePlanefromPointandNormal _grid_center_location "0.000000,0.000000,1.000000"))
  (bind (_worldlocation _worlddirection) (Game|Player|ConvertMouseLocationToWorldSpace _returnvalue))
  (bind _returnvalue_3 (* _worlddirection 1e+04))
  (bind _returnvalue_4 (+ _worldlocation _returnvalue_3))
  (bind (_t _intersection _returnvalue_5) (Class|KismetMathLibrary|LinePlaneIntersection _worldlocation _returnvalue_4 _returnvalue_2))
  (if _returnvalue_5
    (return _intersection)
    (else
      (return "-999.000000,-999.000000,-999.000000"))))

(fn FGetTileIndexfromWorldLocation
  (params (Location :type Vector))
  (Utilities|FlowControl|Sequence
    (:then_0
      (LocalVariables|SetLocationOnGrid (- Location (Variables|Default|GetGrid%20Bottom%20Left%20Corner%20Location)))
      (LocalVariables|SetSnappedLocationOnGrid (Math|Conversions|ToVector2D(Vector) (CallFunction|FSnapVectortoVector (* (LocalVariables|GetLocationOnGrid) "1.000000,2.000000,1.000000") (* (Variables|Default|GetGrid%20Tile%20Size) "0.750000,0.250000,1.000000"))))
      (LocalVariables|SetTempIndex (/ (LocalVariables|GetSnappedLocationOnGrid) (* (Math|Conversions|ToVector2D(Vector) (Variables|Default|GetGrid%20Tile%20Size)) "(X=0.750000,Y=1.000000)")))
      (if (CallFunction|FIsFloatEven (.x (LocalVariables|GetTempIndex)))
        (LocalVariables|SetRetIndex (Utilities|Struct|MakeIntPoint (Math|Float|Truncate (.x (LocalVariables|GetTempIndex))) (* (Math|Float|Round (/ (.y (LocalVariables|GetTempIndex)) 2.0)) 2)))
        (else
          (LocalVariables|SetRetIndex (Utilities|Struct|MakeIntPoint (Math|Float|Truncate (.x (LocalVariables|GetTempIndex))) (+ (* (Math|Float|Floor (/ (.y (LocalVariables|GetTempIndex)) 2.0)) 2) 1))))))
    (:then_1
      (return (LocalVariables|GetRetIndex)))))